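; Game instance that owns the LAN party manager and announces this game's presence on the local network.
; On Init it constructs a LanPartyManager object outered to itself and starts a looping half-second timer that has the manager broadcast a discovery message.
; On Shutdown it clears that timer and tells the manager to leave the party.
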(event Custom|BroadCastDiscoveryMessage
  ;[1 1 1 0] Announce presence on network
  (Class|LanPartyManager|BroadcastDiscoveryMessage (Variables|Default|GetPartyManager)))

(event EventShutdown
  ;[1 1 1 0] Cleanup
  (Utilities|Time|ClearandInvalidateTimerbyHandle (Variables|Default|GetBroadcastDiscoveryTimer))
  (Class|LanPartyManager|LeaveParty (Variables|Default|GetPartyManager)))

(event EventInit
  ;[1 1 1 0] Construct LanPartyManager UObject
  (bind _returnvalue (Game|ConstructObjectfromClass "/Script/LanParty.LanPartyManager" self))
  (Variables|Default|SetPartyManager _returnvalue)
  (bind _returnvalue_2 (Utilities|Time|SetTimerbyEvent (delegate Custom|BroadCastDiscoveryMessage) 0.5 true))
  (Variables|Default|SetBroadcastDiscoveryTimer _returnvalue_2))