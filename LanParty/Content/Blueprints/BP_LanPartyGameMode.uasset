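; LAN party lobby game mode that matches players and launches a listen-server game.
; It shows the lobby widget and binds PartyManager delegates from the game instance; each join restarts the matchmaking timer.
; On timeout or skip, the host opens GameMap as listen server; clients join on the server-ready address (port 7777), with a timed error message.
; Debug keys join, leave, skip and quit; Tick prints party state.
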(event Custom|OnPlayerJoinedParty
  (params (PlayerIndex :type Byte))
  (CallFunction|StartMatchmaking) ; Reset our timer when another player joins party
)

(event Custom|OnSkipCountdown
  (CallFunction|OnMatchmakingComplete))

(event Custom|OnServerReady
  (params (ServerAddress :type String))
  (CallFunction|JoinServer ServerAddress))

(event EventTick
  (params (DeltaSeconds :type Float%20%28single-precision%29))
  (bind _partymanager (Variables|Default|GetPartyManager))
  ;[1 1 1 0] Debug
  (Development|PrintText (Utilities|Text|FormatText "PlayerIndex = {PlayerIndex}" (Variables|/Script/LanParty.LanPartyManager|GetPlayerIndex (Variables|Default|GetPartyManager))) true false "(R=1.000000,G=1.000000,B=1.000000,A=1.000000)" 0.0)
  (Class|LanPartyManager|PrintPartyInfo _partymanager)
  (Development|PrintText (Utilities|Text|FormatText "Match Start Time: {Match Start Time}" (Class|KismetTextLibrary|AsTimeDateTime (Variables|/Script/LanParty.LanPartyManager|GetMatchStartTime _partymanager))) true false "(R=1.000000,G=1.000000,B=1.000000,A=1.000000)" 0.0))

(event EventBeginPlay
  (bind _returnvalue (Game|GetPlayerController 0))
  ;[1 1 1 0] Init UI
  (Input|EnableInput _returnvalue)
  (bind _returnvalue_2 (UserInterface|CreateWidget "/LanParty/Blueprints/BPW_LanPartyLobby.BPW_LanPartyLobby_C" _returnvalue))
  (UserInterface|Viewport|AddtoViewport _returnvalue_2 0)
  (bind _asbp_lan_party_game_instance (Utilities|Casting|CastToBP_LanPartyGameInstance (Game|GetGameInstance)))
  (Variables|Default|SetPartyManager (Variables|/LanParty/Blueprints/BP_LanPartyGameInstance.BP_LanPartyGameInstance_C|GetPartyManager _asbp_lan_party_game_instance))
  (Utilities|FlowControl|Sequence
    (:then_0
      (EventDispatchers|BindEventtoSkipCountdownDelegate (Variables|Default|GetPartyManager) (delegate Custom|OnSkipCountdown)))
    (:then_1
      (EventDispatchers|BindEventtoServerReadyDelegate (Variables|Default|GetPartyManager) (delegate Custom|OnServerReady)))
    (:then_2
      (EventDispatchers|BindEventtoPlayerJoinedPartyDelegate (Variables|Default|GetPartyManager) (delegate Custom|OnPlayerJoinedParty)))))

(event Input|KeyboardEvents|SpaceBar
  (params (Key :type Key%20Structure))
  ;[1 1 1 0] Debug
  (:Pressed
    (if (Class|LanPartyManager|IsinParty (Variables|Default|GetPartyManager))
      (Class|LanPartyManager|SkipCountdown (Variables|Default|GetPartyManager))
      (CallFunction|OnMatchmakingComplete))))

(event Input|KeyboardEvents|Enter
  (params (Key :type Key%20Structure))
  ;[1 1 1 0] Debug
  (:Pressed
    (if (not (Class|LanPartyManager|IsinParty (Variables|Default|GetPartyManager)))
      (Class|LanPartyManager|JoinParty (Variables|Default|GetPartyManager))
      (CallFunction|StartMatchmaking))))

(event Input|KeyboardEvents|Escape
  (params (Key :type Key%20Structure))
  ;[1 1 1 0] Debug
  (:Pressed
    (Game|QuitGame 0 "Quit" false)))

(event Input|KeyboardEvents|Q
  (params (Key :type Key%20Structure))
  ;[1 1 1 0] Debug
  (:Pressed
    (if (Class|LanPartyManager|IsinParty (Variables|Default|GetPartyManager))
      (Class|LanPartyManager|LeaveParty (Variables|Default|GetPartyManager))
      (Utilities|Time|ClearandInvalidateTimerbyHandle (Variables|Default|GetMatchmakingTimer)))))

(fn ConstructionScript)

(fn OnMatchmakingComplete
  (if (Class|LanPartyManager|IsinParty (Variables|Default|GetPartyManager))
    (bind _returnvalue (Class|LanPartyManager|CheckIsGameHost (Variables|Default|GetPartyManager)))
    (if _returnvalue
      (Game|OpenLevel(byName) "GameMap" true "listen")
      (else
        (Utilities|Time|SetTimerbyFunctionName 0 "OnServerJoinError" 5.0)))
    (return)))

(fn OnServerJoinError
  (Development|PrintString "Error Joining Server" true true "(R=1.000000,G=0.000000,B=0.016751,A=1.000000)" 15.0)
  (return))

(fn JoinServer
  (params (IpAddress :type String))
  (Game|OpenLevel(byName) (Utilities|String|StringToName (Utilities|String|JoinStringArray (Utilities|Array|MakeArray IpAddress "7777") ":")))
  (return))

(fn StartMatchmaking
  (bind _returnvalue (Utilities|Time|SetTimerbyFunctionName 0 "OnMatchmakingComplete" (Math|Conversions|ToFloat(Integer) (Variables|/Script/LanParty.LanPartyManager|GetMatchmakingLengthSeconds (Variables|Default|GetPartyManager)))))
  (Variables|Default|SetMatchmakingTimer _returnvalue)
  (return))